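; System Blueprint that turns text into 3D letter characters and manages their camera view and color, adding the W_Edit_Misaki widget at startup.
; CreateCharactor blends the camera to a random BP_SpawnArea and spawns one BP_Letter_Misaki per character in a Y-offset row, assigning each an animation Blueprint.
; CameraChange re-picks a random area for the view.
; LetterColorChange swaps materials on the last spawned letters by color name.
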(event Custom|CreateCharactor
  (params (Text :type String))
  (Utilities|Array|Clear (Variables|Default|GetLastLetters))
  (bind _outactors (Actor|GetAllActorsOfClass "/Game/Inoue/BP/BPS/BP_SpawnArea.BP_SpawnArea_C"))
  (bind _output_get (Variables|Default|SetLastSpawnArea (Utilities|Array|Get(acopy) _outactors (Math|Random|RandomIntegerinRange 0 (- (Utilities|Array|Length _outactors) 1)))))
  (Variables|Default|SetSpotTransform (Transformation|GetActorTransform _output_get))
  (Game|Player|SetViewTargetwithBlend (Game|GetPlayerController 0) (Variables|Default|GetLastSpawnArea) 1.0 "VTBlend_EaseInOut" 2.0 false) ; カメラ切り替え
  (for _index (range 0 (- (Utilities|String|Len Text) 1))
    (bind _returnvalue (Game|SpawnActorfromClass "/Game/Inoue/BP/BPS/BP_Letter_Misaki.BP_Letter_Misaki_C" (Math|Transform|MakeTransform (Math|Vector|MakeVector (.X (Math|Vector|BreakVector (.location (Variables|Default|GetSpotTransform)))) (+ (.Y (Math|Vector|BreakVector (.location (Variables|Default|GetSpotTransform)))) (* _index 85)) (.Z (Math|Vector|BreakVector (.location (Variables|Default|GetSpotTransform))))) (.rotation (Variables|Default|GetSpotTransform)) (.scale (Variables|Default|GetSpotTransform))) "Undefined" "MultiplyWithRoot" 0 (Utilities|String|Left (Class|KismetStringLibrary|Mid Text _index 1) 1) 0))
    (Utilities|Array|Add (Variables|Default|GetLastLetters) _returnvalue)
    (Class|SkeletalMeshComponent|SetAnimClass (Variables|/Game/Inoue/BP/BPS/BP_Letter_Misaki.BP_Letter_Misaki_C|GetBody _returnvalue) "/Game/Inoue/BP/SK_TM_I_AnimBlueprint.SK_TM_I_AnimBlueprint_C")))

(event Custom|LetterColorChange
  (params (ColorName :type String))
  (for _array_element (Variables|Default|GetLastLetters)
    (switch string ColorName
      (:Default
        (Rendering|Material|CreateDynamicMaterialInstance (Variables|/Game/Inoue/BP/BPS/BP_Letter_Misaki.BP_Letter_Misaki_C|GetBody _array_element) 0 "/Game/Inoue/BasicShapeMaterial.BasicShapeMaterial" "None" :!class /Script/Engine.PrimitiveComponent))
      (:Green
        (Rendering|Material|CreateDynamicMaterialInstance (Variables|/Game/Inoue/BP/BPS/BP_Letter_Misaki.BP_Letter_Misaki_C|GetBody _array_element) 0 "/Game/Inoue/MyStuff/Material/M_Text_Color_Gr.M_Text_Color_Gr" "None" :!class /Script/Engine.PrimitiveComponent))
      (:Orange
        (Rendering|Material|CreateDynamicMaterialInstance (Variables|/Game/Inoue/BP/BPS/BP_Letter_Misaki.BP_Letter_Misaki_C|GetBody _array_element) 0 "/Game/Inoue/MyStuff/Material/M_Text_Color_Or.M_Text_Color_Or" "None" :!class /Script/Engine.PrimitiveComponent))
      (:Yellow
        (Rendering|Material|CreateDynamicMaterialInstance (Variables|/Game/Inoue/BP/BPS/BP_Letter_Misaki.BP_Letter_Misaki_C|GetBody _array_element) 0 "/Game/Inoue/MyStuff/Material/M_Text_Color_Yel.M_Text_Color_Yel" "None" :!class /Script/Engine.PrimitiveComponent))
      (:Blue
        (Rendering|Material|CreateDynamicMaterialInstance (Variables|/Game/Inoue/BP/BPS/BP_Letter_Misaki.BP_Letter_Misaki_C|GetBody _array_element) 0 "/Game/Inoue/MyStuff/Material/M_Text_Color_Blu.M_Text_Color_Blu" "None" :!class /Script/Engine.PrimitiveComponent))
      (:Purple
        (Rendering|Material|CreateDynamicMaterialInstance (Variables|/Game/Inoue/BP/BPS/BP_Letter_Misaki.BP_Letter_Misaki_C|GetBody _array_element) 0 "/Game/Inoue/MyStuff/Material/M_Text_Color_Pur.M_Text_Color_Pur" "None" :!class /Script/Engine.PrimitiveComponent))
      (:Pink
        (Rendering|Material|CreateDynamicMaterialInstance (Variables|/Game/Inoue/BP/BPS/BP_Letter_Misaki.BP_Letter_Misaki_C|GetBody _array_element) 0 "/Game/Inoue/MyStuff/Material/M_Text_Color_Pink.M_Text_Color_Pink" "None" :!class /Script/Engine.PrimitiveComponent))
      (:Gray
        (Rendering|Material|CreateDynamicMaterialInstance (Variables|/Game/Inoue/BP/BPS/BP_Letter_Misaki.BP_Letter_Misaki_C|GetBody _array_element) 0 "/Game/Inoue/MyStuff/Material/M_Text_Color_Gry.M_Text_Color_Gry" "None" :!class /Script/Engine.PrimitiveComponent)))))

(event Custom|ColorChangeY)

(event Custom|ColorChangeO)

(event Custom|CameraChange
  (for (_ _array_index) (Utilities|Array|MakeArray (Variables|Default|GetLastSpawnArea))
    (bind _outactors (Actor|GetAllActorsOfClass "/Game/Inoue/BP/BPS/BP_SpawnArea.BP_SpawnArea_C"))
    (bind _output_get (Variables|Default|SetLastSpawnArea (Utilities|Array|Get(acopy) _outactors (Math|Random|RandomIntegerinRange 0 (- (Utilities|Array|Length _outactors) 1)))))
    (Variables|Default|SetSpotTransform (Transformation|GetActorTransform _output_get))
    (Game|Player|SetViewTargetwithBlend (Game|GetPlayerController _array_index) (Variables|Default|GetLastSpawnArea) 1.0 "VTBlend_EaseInOut" 2.0 false) ; カメラ切り替え
  ))

(event Custom|PlayAnim)

(event EventBeginPlay
  (bind _returnvalue (UserInterface|CreateWidget "/Game/Inoue/BP/BPS/W_Edit_Misaki.W_Edit_Misaki_C"))
  (bind _output_get (Variables|Default|SetWidgetEdit2 _returnvalue))
  (UserInterface|Viewport|AddtoViewport _output_get 0))

(event Collision|EventActorBeginOverlap
  (params (OtherActor :type Actor%20Object%20Reference)))

(event EventTick
  (params (DeltaSeconds :type Float%20%28single-precision%29)))

(fn ConstructionScript)