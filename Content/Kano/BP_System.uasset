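; BP_System is an actor that sets up a text-edit UI and spawns letter characters into the level.
; On BeginPlay it creates a W_Edit widget, stores it and adds it to the viewport.
; Its CreateCharacter event picks a random BP_SpawnArea actor and spawns a BP_Letter_Kano at that transform, passing the first character of the given text as its Letter.
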(event Custom|CreateCharacter
  (params (Text :type String))
  (bind _outactors (Actor|GetAllActorsOfClass "/Game/Inoue/BP/BPS/BP_SpawnArea.BP_SpawnArea_C"))
  (Game|SpawnActorfromClass "/Game/Kano/BP_Letter_Kano.BP_Letter_Kano_C" (Transformation|GetActorTransform (Utilities|Array|Get(acopy) _outactors (Math|Random|RandomIntegerinRange 0 (- (Utilities|Array|Length _outactors) 1)))) "Undefined" "MultiplyWithRoot" 0 (Utilities|String|Left Text 1) 0))

(event EventBeginPlay
  (bind _returnvalue (UserInterface|CreateWidget "/Game/Kano/W_Edit.W_Edit_C"))
  (bind _output_get (Variables|Default|SetWidget_Edit _returnvalue))
  (UserInterface|Viewport|AddtoViewport _output_get 0))

(event Collision|EventActorBeginOverlap
  (params (OtherActor :type Actor%20Object%20Reference)))

(event EventTick
  (params (DeltaSeconds :type Float%20%28single-precision%29)))

(fn ConstructionScript)